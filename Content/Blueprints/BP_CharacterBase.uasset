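; Base character Blueprint that colors a modular fantasy hero from its customization choices at BeginPlay.
; SetMaterials creates a dynamic material instance on the skeletal mesh and assigns a base mesh and material to Mask.
; CharacterCustomizationComponent selections become clamped indices into color arrays that feed the material's vector parameters, with skin choice also driving stubble and scar colors.
; A touch-enter event only prints a greeting.
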(event `self.ReceiveBeginPlay`
  (`self.SetMaterials`))

(event `self.ReceiveActorOnInputTouchEnter`
  (params (FingerIndex :type "ETouchIndex Enum" :default "Touch1"))
  (`KismetSystemLibrary.PrintString` "Hello"))

(fn `SetMaterials`
  (bind _colors_leatherprimarycolor_ar (`self.Colors_LeatherPrimaryColor_ar`))
  (bind _colors_skincolor_ar (`self.Colors_SkinColor_ar`))
  (bind _dynamicmaterial (`self.DynamicMaterial`))
  (bind _charactercustomizationcomponent (`self.CharacterCustomizationComponent`))
  (bind _mask (`self.Mask`))
  (bind _colors_leathersecondarycolor_ar (`self.Colors_LeatherSecondaryColor_ar`))
  (bind _colors_secondarycolor_ar (`self.Colors_SecondaryColor_ar`))
  (bind _colors_metalprimarycolor_ar (`self.Colors_MetalPrimaryColor_ar`))
  (bind _colors_metalsecondarycolor_ar (`self.Colors_MetalSecondaryColor_ar`))
  (bind _colors_metaldarkcolor_ar (`self.Colors_MetalDarkColor_ar`))
  (bind _colors_bodyartcolor_ar (`self.Colors_BodyArtColor_ar`))
  (bind _colors_haircolor_ar (`self.Colors_HairColor_ar`))
  (bind _colors_primarycolor_ar (`self.Colors_PrimaryColor_ar`))
  (bind _returnvalue (`KismetMathLibrary.Clamp` (`KismetMathLibrary.Conv_ByteToInt` (`CharacterCustomizationComponent.ColorSkin` _charactercustomizationcomponent)) 0 (`KismetArrayLibrary.Array_LastIndex` _colors_skincolor_ar)))
  (bind _returnvalue_2 (`PrimitiveComponent.CreateDynamicMaterialInstance` (`self.SkeletalMesh`) 0 "/Game/_Resources/ModularCharacters/Materials/ModularFantasyHeroCharacters.ModularFantasyHeroCharacters" "None"))
  (set `self.DynamicMaterial` _returnvalue_2)
  (`SkinnedMeshComponent.SetSkinnedAssetAndUpdate` _mask "/Game/Characters/Modular/Meshes/SKM_Polygon_Base.SKM_Polygon_Base" true)
  (`PrimitiveComponent.SetMaterial` _mask 0 "/Game/_Resources/ModularCharacters/Materials/Mask.Mask")
  ;[1 1 1] Material_Color_Skin
  (`MaterialInstanceDynamic.SetVectorParameterValue` _dynamicmaterial "Color_Skin" (`|GetArrayItem` _colors_skincolor_ar _returnvalue))
  ;[1 1 1] Material_Color_Stubble
  (`MaterialInstanceDynamic.SetVectorParameterValue` _dynamicmaterial "Color_Stubble" (`|GetArrayItem` (`self.Colors_StubbleColor_ar`) _returnvalue))
  ;[1 1 1] Material_Color_Scar
  (`MaterialInstanceDynamic.SetVectorParameterValue` _dynamicmaterial "Color_Scar" (`|GetArrayItem` (`self.Colors_ScarColor_ar`) _returnvalue))
  ;[1 1 1] Material_Color_Primary
  (`MaterialInstanceDynamic.SetVectorParameterValue` _dynamicmaterial "Color_Primary" (`|GetArrayItem` _colors_primarycolor_ar (`KismetMathLibrary.Clamp` (`KismetMathLibrary.Conv_ByteToInt` (`CharacterCustomizationComponent.ColorPrimary` _charactercustomizationcomponent)) 0 (`KismetArrayLibrary.Array_LastIndex` _colors_primarycolor_ar))))
  ;[1 1 1] Material_Color_Secondary
  (`MaterialInstanceDynamic.SetVectorParameterValue` _dynamicmaterial "Color_Secondary" (`|GetArrayItem` _colors_secondarycolor_ar (`KismetMathLibrary.Clamp` (`KismetMathLibrary.Conv_ByteToInt` (`CharacterCustomizationComponent.ColorSecondary` _charactercustomizationcomponent)) 0 (`KismetArrayLibrary.Array_LastIndex` _colors_secondarycolor_ar))))
  ;[1 1 1] Material_MetalPrimaryColor
  (`MaterialInstanceDynamic.SetVectorParameterValue` _dynamicmaterial "Color_Metal_Primary" (`|GetArrayItem` _colors_metalprimarycolor_ar (`KismetMathLibrary.Clamp` (`KismetMathLibrary.Conv_ByteToInt` (`CharacterCustomizationComponent.ColorMetalPrimary` _charactercustomizationcomponent)) 0 (`KismetArrayLibrary.Array_LastIndex` _colors_metalprimarycolor_ar))))
  ;[1 1 1] Material_MetalSecondaryColor
  (`MaterialInstanceDynamic.SetVectorParameterValue` _dynamicmaterial "Color_Metal_Secondary" (`|GetArrayItem` _colors_metalsecondarycolor_ar (`KismetMathLibrary.Clamp` (`KismetMathLibrary.Conv_ByteToInt` (`CharacterCustomizationComponent.ColorMetalSecondary` _charactercustomizationcomponent)) 0 (`KismetArrayLibrary.Array_LastIndex` _colors_metalsecondarycolor_ar))))
  ;[1 1 1] Material_MetalDarkColor
  (`MaterialInstanceDynamic.SetVectorParameterValue` _dynamicmaterial "Color_Metal_Dark" (`|GetArrayItem` _colors_metaldarkcolor_ar (`KismetMathLibrary.Clamp` (`KismetMathLibrary.Conv_ByteToInt` (`CharacterCustomizationComponent.ColorMetalDark` _charactercustomizationcomponent)) 0 (`KismetArrayLibrary.Array_LastIndex` _colors_metaldarkcolor_ar))))
  ;[1 1 1] Material_LeatherPrimaryColor
  (`MaterialInstanceDynamic.SetVectorParameterValue` _dynamicmaterial "Color_Leather_Primary" (`|GetArrayItem` _colors_leatherprimarycolor_ar (`KismetMathLibrary.Clamp` (`KismetMathLibrary.Conv_ByteToInt` (`CharacterCustomizationComponent.ColorLeatherPrimary` _charactercustomizationcomponent)) 0 (`KismetArrayLibrary.Array_LastIndex` _colors_leatherprimarycolor_ar))))
  ;[1 1 1] Material_LeatherPrimaryColor
  (`MaterialInstanceDynamic.SetVectorParameterValue` _dynamicmaterial "Color_Leather_Secondary" (`|GetArrayItem` _colors_leathersecondarycolor_ar (`KismetMathLibrary.Clamp` (`KismetMathLibrary.Conv_ByteToInt` (`CharacterCustomizationComponent.ColorLeatherSecondary` _charactercustomizationcomponent)) 0 (`KismetArrayLibrary.Array_LastIndex` _colors_leathersecondarycolor_ar))))
  ;[1 1 1] Material_Hair
  (`MaterialInstanceDynamic.SetVectorParameterValue` _dynamicmaterial "Color_Hair" (`|GetArrayItem` _colors_haircolor_ar (`KismetMathLibrary.Clamp` (`KismetMathLibrary.Conv_ByteToInt` (`CharacterCustomizationComponent.ColorHair` _charactercustomizationcomponent)) 0 (`KismetArrayLibrary.Array_LastIndex` _colors_haircolor_ar))))
  ;[1 1 1] Material_BodyArtColor
  (`MaterialInstanceDynamic.SetVectorParameterValue` _dynamicmaterial "Color_BodyArt" (`|GetArrayItem` _colors_bodyartcolor_ar (`KismetMathLibrary.Clamp` (`KismetMathLibrary.Conv_ByteToInt` (`CharacterCustomizationComponent.ColorBodyArt` _charactercustomizationcomponent)) 0 (`KismetArrayLibrary.Array_LastIndex` _colors_bodyartcolor_ar)))))

(fn `UserConstructionScript`)